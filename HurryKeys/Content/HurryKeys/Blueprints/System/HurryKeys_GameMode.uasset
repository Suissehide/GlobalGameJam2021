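; HurryKeys game mode that runs the countdown timer, tracks the key and creates the game UI.
; While Start is set, Tick uses a one-second Delay to count down seconds and roll over minutes.
; When minutes drop below zero, it clears Start and calls PlayerLose on the player's MichelleCharacter.
; Separate events add the UI_game widget to the viewport and set Key to 1, rather than incrementing it.
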(event `createUI`
  (bind _returnvalue (`|CreateWidget` "/Game/HurryKeys/Blueprints/Interfaces/UI_game.UI_game_C"))
  (`UserWidget.AddToViewport` _returnvalue 0))

(event `self.ReceiveBeginPlay`)

(event `self.ReceiveTick`
  (params (DeltaSeconds :type "Float (single-precision)"))
  (if (`self.start`)
    (`KismetSystemLibrary.Delay` 1.0)
    (set `self.TimeSec` (- (`self.TimeSec`) 1))
    (if (<= (`self.TimeSec`) 0)
      (set `self.TimeMin` (- (`self.TimeMin`) 1))
      (set `self.TimeSec` 59)
      (if (< (`self.TimeMin`) 0)
        (set `self.start` false)
        (bind _asmichelle_character (cast `/Game/HurryKeys/Blueprints/Characters/Michelle/MichelleCharacter` (`GameplayStatics.GetPlayerCharacter` 0)))
        (`/Game/HurryKeys/Blueprints/Characters/Michelle/MichelleCharacter.playerLose` _asmichelle_character)))))

(event `addKey`
  (set `self.Key` 1))

(fn `UserConstructionScript`)